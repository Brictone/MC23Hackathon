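; SMG item for a hand-grip interaction system, with two-handed aiming.
; SCLogicSetup registers four sub-components: physics frame as primary grip, an X-axis sliding part, a magwell attachment point and a foregrip.
; While a locally controlled pawn holds the foregrip, Tick re-aims the frame's solid hand between both ghost palms, pinning it to the primary palm and projecting the foregrip palm onto a forward plane.
; Construction Script prints a debug palm offset.
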(event EventBeginPlay
  (|CallParentFunction) ; This node is disabled and will not be called.\nDrag off pins to build functionality.
)

(event Collision|EventActorBeginOverlap
  (params (OtherActor :type Actor%20Object%20Reference))
  (|CallParentFunction OtherActor) ; This node is disabled and will not be called.\nDrag off pins to build functionality.
)

(event EventTick
  (params (DeltaSeconds :type Float%20%28single-precision%29))
  (bind _subcomponentmap (Variables|Default|GetSubComponentMap))
  (bind _capsule (Variables|Default|GetCapsule))
  (bind _value (Utilities|Map|Find _subcomponentmap _capsule))
  (bind _state (Utilities|Struct|BreakSTRUCT_21_SubComponentLogic _value))
  (bind (_busygrip_ _held_ _beingmanipulated_ _manipulationcalcs _hand) (Utilities|Struct|BreakStruct_21_ComponentState _state))
  (|CallParentFunction DeltaSeconds)
  (Utilities|FlowControl|Sequence
    (:then_0
      (if _beingmanipulated_
        (bind _aspawn (Utilities|Casting|CastToPawn (.Pawn (Utilities|Struct|BreakStruct_21_HandSingularity _hand))))
        (if (Pawn|IsLocallyControlled _aspawn)
          (CallFunction|NewFunction00 _value))))))

(event EventSCLogicSetup
  (bind _0_mesh_base (Variables|Default|Get0_Mesh_Base))
  (bind _staticmesh1 (Variables|Default|GetStaticMesh1))
  (bind _capsule (Variables|Default|GetCapsule))
  (bind _capsule2 (Variables|Default|GetCapsule2))
  (Utilities|FlowControl|Sequence
    (:then_0
      (Utilities|FlowControl|Sequence
        (:then_0
          (Utilities|Map|Add (Variables|Default|GetSubComponentMap) _0_mesh_base (Utilities|Struct|MakeSTRUCT_21_SubComponentLogic (Utilities|Struct|MakeStruct_21_SubComponentObjects (Variables|Default|Get0_Mesh_Base) _0_mesh_base (Variables|Default|Get0_HandScene) (Variables|Default|Get0_Highlighter) self (Variables|Default|Get0_HandMesh)) (Utilities|Struct|MakeStruct_21_BasicComponentBehavior true "NewEnumerator0" false false false false false false false "NewEnumerator0" true) "(Movable?_1_F18DBC344390B161DCD264B196928299=False,Button?_9_D4AE62AB4386BC3CB9F0ADA62143FBAC=False,MustHoldPrimary?_5_E662F56A44D8AAF8C5393F951F7F74EC=False,MovementConstraints_6_A626FB894F5E9C4E7FBE1E9E92EB0E13=(LinearRelativeSpace_23_57B6E833477E786761A080957E953B34=NewEnumerator1,Button_31_0730DB4C4B036A5886FE15B828FFFEE3=(Toggleable?_3_35007B1949ABC9888873D4866C35477C=False,Sticky?_21_C890B630443EEB468DFF28843F253075=False,MinX_9_0FF88DFE4217FFF1EC905BB447CBF3B2=0.000000,MaxX_8_B370D57E443F5E0E24FDDABA0BA99C7D=0.000000,ResetX_11_5B812BFE4FD86D460FEE8198946B7B57=0.000000,ToggleX_13_DA5536974CA964836CF06BB91D709D40=0.000000,ActiveToggleOnThresh_15_E7080EA6454858B5DC8A948E40BC5BC1=0.000000,ToggleOffThresh_17_2D36698647CF2A7BF48E7FAB9BFEB092=0.000000,Speed_19_6497B3894B3DAA00D8E02C96A6FBEDC0=10.000000,SceneDelta_27_25CC51834345C2987CDFF4872ACA290A=0.000000,Axis_24_4F466FBC492CB3E26EA5AEA588AC7F1E=NewEnumerator1),X_6_4CF1D35C4D6BDC63300BA2850D0DA911=(BoundsType_3_295CD98E4D2862A6B4052790986A46EA=NewEnumerator0,LockSpecifiedValue_5_1E8FC7F64E9F7D85E5F24A85E78A6CFA=0.000000,Min_7_2A1EBA064A0EA8126606B59CD598994E=0.000000,Max_9_CD75696C42CE808B0A8BE1B2E7D1E63E=0.000000,ResetOnDrop?_14_B5062806488C4B3CFA94728FF0322F7D=True),Y_7_9326C9DE464AA7532AC664ABEB0B4BD4=(BoundsType_3_295CD98E4D2862A6B4052790986A46EA=NewEnumerator0,LockSpecifiedValue_5_1E8FC7F64E9F7D85E5F24A85E78A6CFA=0.000000,Min_7_2A1EBA064A0EA8126606B59CD598994E=0.000000,Max_9_CD75696C42CE808B0A8BE1B2E7D1E63E=0.000000,ResetOnDrop?_14_B5062806488C4B3CFA94728FF0322F7D=True),Z_8_55932C074E62FF028752F49130D36B1E=(BoundsType_3_295CD98E4D2862A6B4052790986A46EA=NewEnumerator0,LockSpecifiedValue_5_1E8FC7F64E9F7D85E5F24A85E78A6CFA=0.000000,Min_7_2A1EBA064A0EA8126606B59CD598994E=0.000000,Max_9_CD75696C42CE808B0A8BE1B2E7D1E63E=0.000000,ResetOnDrop?_14_B5062806488C4B3CFA94728FF0322F7D=True),Roll_18_CE1BEC3D44CB2BB950A8CF8D3F9ECAF9=(BoundsType_3_295CD98E4D2862A6B4052790986A46EA=NewEnumerator0,LockSpecifiedValue_5_1E8FC7F64E9F7D85E5F24A85E78A6CFA=0.000000,Min_7_2A1EBA064A0EA8126606B59CD598994E=0.000000,Max_9_CD75696C42CE808B0A8BE1B2E7D1E63E=0.000000,HandAxisBinding_15_7791594F48674BE9C9DB8A83B34E0C75=NewEnumerator1,ResetOnDrop?_17_54497A634287FD69CB6B0ABA09C6D891=True),Pitch_15_75ADFC1746D100E93400C4BD39AAB82A=(BoundsType_3_295CD98E4D2862A6B4052790986A46EA=NewEnumerator0,LockSpecifiedValue_5_1E8FC7F64E9F7D85E5F24A85E78A6CFA=0.000000,Min_7_2A1EBA064A0EA8126606B59CD598994E=0.000000,Max_9_CD75696C42CE808B0A8BE1B2E7D1E63E=0.000000,HandAxisBinding_15_7791594F48674BE9C9DB8A83B34E0C75=NewEnumerator0,ResetOnDrop?_17_54497A634287FD69CB6B0ABA09C6D891=True),Yaw_19_B0B70B5C4A9B6D67D99480B858D58622=(BoundsType_3_295CD98E4D2862A6B4052790986A46EA=NewEnumerator0,LockSpecifiedValue_5_1E8FC7F64E9F7D85E5F24A85E78A6CFA=0.000000,Min_7_2A1EBA064A0EA8126606B59CD598994E=0.000000,Max_9_CD75696C42CE808B0A8BE1B2E7D1E63E=0.000000,HandAxisBinding_15_7791594F48674BE9C9DB8A83B34E0C75=NewEnumerator2,ResetOnDrop?_17_54497A634287FD69CB6B0ABA09C6D891=True),Radial_28_898129014273BCFB5591F487B2C04056=(Enable?_8_FF416EB24FD6F69B1E11489EA5FD45DB=False,FreeAxis_2_C3F822154C66E04357E4899DCCC46DD3=NewEnumerator2,PolarOrigin_5_9ACA6D4D4576C593C6399CAA9C469075=None,Pointer_13_7260199B49F9A60A0DB5869F3F30E66D=None,ResetOnDrop?_10_7C4F98834A8F576AD1C7049B7BEAA6C3=True)),Prox?_11_91C50ED9429A218EE873CBAC54F573CA=False)" (Utilities|Struct|MakeStruct_21_GripInfo "0.000000,0.000000,0.000000|0.000000,0.000000,0.000000|1.000000,1.000000,1.000000" false "NewEnumerator1" "NewEnumerator0" 0.0 "NewEnumerator1"))))
        (:then_1
          (Utilities|Map|Add (Variables|Default|GetSubComponentMap) _staticmesh1 (Utilities|Struct|MakeSTRUCT_21_SubComponentLogic (Utilities|Struct|MakeStruct_21_SubComponentObjects (Variables|Default|GetScene2) _staticmesh1 (Variables|Default|GetScene3) (Variables|Default|GetCapsule1) self (Variables|Default|GetSkeletalMesh1)) (Utilities|Struct|MakeStruct_21_BasicComponentBehavior false "NewEnumerator1" true) (Utilities|Struct|MakeStruct_21_ManipulationOptions true false true (Utilities|Struct|MakeStruct_ConstraintContainer "NewEnumerator1" "(Toggleable?_3_35007B1949ABC9888873D4866C35477C=False,Sticky?_21_C890B630443EEB468DFF28843F253075=False,MinX_9_0FF88DFE4217FFF1EC905BB447CBF3B2=0.000000,MaxX_8_B370D57E443F5E0E24FDDABA0BA99C7D=0.000000,ResetX_11_5B812BFE4FD86D460FEE8198946B7B57=0.000000,ToggleX_13_DA5536974CA964836CF06BB91D709D40=0.000000,ActiveToggleOnThresh_15_E7080EA6454858B5DC8A948E40BC5BC1=0.000000,ToggleOffThresh_17_2D36698647CF2A7BF48E7FAB9BFEB092=0.000000,Speed_19_6497B3894B3DAA00D8E02C96A6FBEDC0=10.000000,SceneDelta_27_25CC51834345C2987CDFF4872ACA290A=0.000000,Axis_24_4F466FBC492CB3E26EA5AEA588AC7F1E=NewEnumerator1)" (Utilities|Struct|MakeStruct_LinearConstraints "NewEnumerator3" 22.0 16.0 22.0) "(BoundsType_3_295CD98E4D2862A6B4052790986A46EA=NewEnumerator0,LockSpecifiedValue_5_1E8FC7F64E9F7D85E5F24A85E78A6CFA=0.000000,Min_7_2A1EBA064A0EA8126606B59CD598994E=0.000000,Max_9_CD75696C42CE808B0A8BE1B2E7D1E63E=0.000000,ResetOnDrop?_14_B5062806488C4B3CFA94728FF0322F7D=True)" "(BoundsType_3_295CD98E4D2862A6B4052790986A46EA=NewEnumerator0,LockSpecifiedValue_5_1E8FC7F64E9F7D85E5F24A85E78A6CFA=0.000000,Min_7_2A1EBA064A0EA8126606B59CD598994E=0.000000,Max_9_CD75696C42CE808B0A8BE1B2E7D1E63E=0.000000,ResetOnDrop?_14_B5062806488C4B3CFA94728FF0322F7D=True)" "(BoundsType_3_295CD98E4D2862A6B4052790986A46EA=NewEnumerator0,LockSpecifiedValue_5_1E8FC7F64E9F7D85E5F24A85E78A6CFA=0.000000,Min_7_2A1EBA064A0EA8126606B59CD598994E=0.000000,Max_9_CD75696C42CE808B0A8BE1B2E7D1E63E=0.000000,HandAxisBinding_15_7791594F48674BE9C9DB8A83B34E0C75=NewEnumerator1,ResetOnDrop?_17_54497A634287FD69CB6B0ABA09C6D891=True)" "(BoundsType_3_295CD98E4D2862A6B4052790986A46EA=NewEnumerator0,LockSpecifiedValue_5_1E8FC7F64E9F7D85E5F24A85E78A6CFA=0.000000,Min_7_2A1EBA064A0EA8126606B59CD598994E=0.000000,Max_9_CD75696C42CE808B0A8BE1B2E7D1E63E=0.000000,HandAxisBinding_15_7791594F48674BE9C9DB8A83B34E0C75=NewEnumerator0,ResetOnDrop?_17_54497A634287FD69CB6B0ABA09C6D891=True)" "(BoundsType_3_295CD98E4D2862A6B4052790986A46EA=NewEnumerator0,LockSpecifiedValue_5_1E8FC7F64E9F7D85E5F24A85E78A6CFA=0.000000,Min_7_2A1EBA064A0EA8126606B59CD598994E=0.000000,Max_9_CD75696C42CE808B0A8BE1B2E7D1E63E=0.000000,HandAxisBinding_15_7791594F48674BE9C9DB8A83B34E0C75=NewEnumerator2,ResetOnDrop?_17_54497A634287FD69CB6B0ABA09C6D891=True)") true) (Utilities|Struct|MakeStruct_21_GripInfo "0.000000,0.000000,0.000000|0.000000,0.000000,0.000000|1.000000,1.000000,1.000000" true "NewEnumerator0" "NewEnumerator1" 1.0 "NewEnumerator3" "NewEnumerator4"))))
        (:then_2
          (Utilities|Map|Add (Variables|Default|GetSubComponentMap) _capsule2 (Utilities|Struct|MakeSTRUCT_21_SubComponentLogic (Utilities|Struct|MakeStruct_21_SubComponentObjects (Variables|Default|GetScene4) _capsule2 (Variables|Default|GetScene5) (Variables|Default|GetCapsule2) self (Variables|Default|GetSkeletalMesh2)) (Utilities|Struct|MakeStruct_21_BasicComponentBehavior false "NewEnumerator2" true) "(Movable?_1_F18DBC344390B161DCD264B196928299=False,Button?_9_D4AE62AB4386BC3CB9F0ADA62143FBAC=False,MustHoldPrimary?_5_E662F56A44D8AAF8C5393F951F7F74EC=False,MovementConstraints_6_A626FB894F5E9C4E7FBE1E9E92EB0E13=(LinearRelativeSpace_23_57B6E833477E786761A080957E953B34=NewEnumerator1,Button_31_0730DB4C4B036A5886FE15B828FFFEE3=(Toggleable?_3_35007B1949ABC9888873D4866C35477C=False,Sticky?_21_C890B630443EEB468DFF28843F253075=False,MinX_9_0FF88DFE4217FFF1EC905BB447CBF3B2=0.000000,MaxX_8_B370D57E443F5E0E24FDDABA0BA99C7D=0.000000,ResetX_11_5B812BFE4FD86D460FEE8198946B7B57=0.000000,ToggleX_13_DA5536974CA964836CF06BB91D709D40=0.000000,ActiveToggleOnThresh_15_E7080EA6454858B5DC8A948E40BC5BC1=0.000000,ToggleOffThresh_17_2D36698647CF2A7BF48E7FAB9BFEB092=0.000000,Speed_19_6497B3894B3DAA00D8E02C96A6FBEDC0=10.000000,SceneDelta_27_25CC51834345C2987CDFF4872ACA290A=0.000000,Axis_24_4F466FBC492CB3E26EA5AEA588AC7F1E=NewEnumerator1),X_6_4CF1D35C4D6BDC63300BA2850D0DA911=(BoundsType_3_295CD98E4D2862A6B4052790986A46EA=NewEnumerator0,LockSpecifiedValue_5_1E8FC7F64E9F7D85E5F24A85E78A6CFA=0.000000,Min_7_2A1EBA064A0EA8126606B59CD598994E=0.000000,Max_9_CD75696C42CE808B0A8BE1B2E7D1E63E=0.000000,ResetOnDrop?_14_B5062806488C4B3CFA94728FF0322F7D=True),Y_7_9326C9DE464AA7532AC664ABEB0B4BD4=(BoundsType_3_295CD98E4D2862A6B4052790986A46EA=NewEnumerator0,LockSpecifiedValue_5_1E8FC7F64E9F7D85E5F24A85E78A6CFA=0.000000,Min_7_2A1EBA064A0EA8126606B59CD598994E=0.000000,Max_9_CD75696C42CE808B0A8BE1B2E7D1E63E=0.000000,ResetOnDrop?_14_B5062806488C4B3CFA94728FF0322F7D=True),Z_8_55932C074E62FF028752F49130D36B1E=(BoundsType_3_295CD98E4D2862A6B4052790986A46EA=NewEnumerator0,LockSpecifiedValue_5_1E8FC7F64E9F7D85E5F24A85E78A6CFA=0.000000,Min_7_2A1EBA064A0EA8126606B59CD598994E=0.000000,Max_9_CD75696C42CE808B0A8BE1B2E7D1E63E=0.000000,ResetOnDrop?_14_B5062806488C4B3CFA94728FF0322F7D=True),Roll_18_CE1BEC3D44CB2BB950A8CF8D3F9ECAF9=(BoundsType_3_295CD98E4D2862A6B4052790986A46EA=NewEnumerator0,LockSpecifiedValue_5_1E8FC7F64E9F7D85E5F24A85E78A6CFA=0.000000,Min_7_2A1EBA064A0EA8126606B59CD598994E=0.000000,Max_9_CD75696C42CE808B0A8BE1B2E7D1E63E=0.000000,HandAxisBinding_15_7791594F48674BE9C9DB8A83B34E0C75=NewEnumerator1,ResetOnDrop?_17_54497A634287FD69CB6B0ABA09C6D891=True),Pitch_15_75ADFC1746D100E93400C4BD39AAB82A=(BoundsType_3_295CD98E4D2862A6B4052790986A46EA=NewEnumerator0,LockSpecifiedValue_5_1E8FC7F64E9F7D85E5F24A85E78A6CFA=0.000000,Min_7_2A1EBA064A0EA8126606B59CD598994E=0.000000,Max_9_CD75696C42CE808B0A8BE1B2E7D1E63E=0.000000,HandAxisBinding_15_7791594F48674BE9C9DB8A83B34E0C75=NewEnumerator0,ResetOnDrop?_17_54497A634287FD69CB6B0ABA09C6D891=True),Yaw_19_B0B70B5C4A9B6D67D99480B858D58622=(BoundsType_3_295CD98E4D2862A6B4052790986A46EA=NewEnumerator0,LockSpecifiedValue_5_1E8FC7F64E9F7D85E5F24A85E78A6CFA=0.000000,Min_7_2A1EBA064A0EA8126606B59CD598994E=0.000000,Max_9_CD75696C42CE808B0A8BE1B2E7D1E63E=0.000000,HandAxisBinding_15_7791594F48674BE9C9DB8A83B34E0C75=NewEnumerator2,ResetOnDrop?_17_54497A634287FD69CB6B0ABA09C6D891=True),Radial_28_898129014273BCFB5591F487B2C04056=(Enable?_8_FF416EB24FD6F69B1E11489EA5FD45DB=False,FreeAxis_2_C3F822154C66E04357E4899DCCC46DD3=NewEnumerator2,PolarOrigin_5_9ACA6D4D4576C593C6399CAA9C469075=None,Pointer_13_7260199B49F9A60A0DB5869F3F30E66D=None,ResetOnDrop?_10_7C4F98834A8F576AD1C7049B7BEAA6C3=True)),Prox?_11_91C50ED9429A218EE873CBAC54F573CA=False)" "(PIckupOffset_12_5ACC95F941AD9A8A6DF52683A8A1737E=(Rotation=(X=0.000000,Y=0.000000,Z=0.000000,W=1.000000),Translation=(X=0.000000,Y=0.000000,Z=0.000000),Scale3D=(X=1.000000,Y=1.000000,Z=1.000000)),Reflection?_14_82FDBA9A41FCD8A869AF619B11559FC1=False,ReflectionAxis_5_B38E55D9470654EFAA6032A8FB977EA2=NewEnumerator1,GripPose_8_182C49484569F8C54CB1AC801069219F=NewEnumerator0,GripStrength_11_5991C4F74DE69A0BDED69A9884AC1F67=0.000000,CollisionOptions_17_BE4BF26943F7E980D264F4AFED50C411=NewEnumerator0,HandManipAttachment_21_1F4E67F34F599384CBFEA3842A4D5AE2=NewEnumerator0,Bone_24_5EC8B0144F76194A0232EAB1BD7F4EDE=\"palmsock\")" (Utilities|Struct|MakeStruct_21_SubAttachOptions "NewEnumerator2" false false true "magwell" "" false (Variables|Default|GetScene4) (Math|Transform|MakeTransform "1.000000, 0,-5.000000" "10.000000, 0, 0") (Variables|Default|GetCapsule2)))))
        (:then_3
          (Utilities|Map|Add (Variables|Default|GetSubComponentMap) _capsule (Utilities|Struct|MakeSTRUCT_21_SubComponentLogic (Utilities|Struct|MakeStruct_21_SubComponentObjects (Variables|Default|GetScene) _capsule (Variables|Default|GetScene1) _capsule self (Variables|Default|GetSkeletalMesh)) (Utilities|Struct|MakeStruct_21_BasicComponentBehavior false "NewEnumerator1" true) (Utilities|Struct|MakeStruct_21_ManipulationOptions false false true (Utilities|Struct|MakeStruct_ConstraintContainer "NewEnumerator1" "(Toggleable?_3_35007B1949ABC9888873D4866C35477C=False,Sticky?_21_C890B630443EEB468DFF28843F253075=False,MinX_9_0FF88DFE4217FFF1EC905BB447CBF3B2=0.000000,MaxX_8_B370D57E443F5E0E24FDDABA0BA99C7D=0.000000,ResetX_11_5B812BFE4FD86D460FEE8198946B7B57=0.000000,ToggleX_13_DA5536974CA964836CF06BB91D709D40=0.000000,ActiveToggleOnThresh_15_E7080EA6454858B5DC8A948E40BC5BC1=0.000000,ToggleOffThresh_17_2D36698647CF2A7BF48E7FAB9BFEB092=0.000000,Speed_19_6497B3894B3DAA00D8E02C96A6FBEDC0=10.000000,SceneDelta_27_25CC51834345C2987CDFF4872ACA290A=0.000000,Axis_24_4F466FBC492CB3E26EA5AEA588AC7F1E=NewEnumerator1)" "(BoundsType_3_295CD98E4D2862A6B4052790986A46EA=NewEnumerator0,LockSpecifiedValue_5_1E8FC7F64E9F7D85E5F24A85E78A6CFA=0.000000,Min_7_2A1EBA064A0EA8126606B59CD598994E=0.000000,Max_9_CD75696C42CE808B0A8BE1B2E7D1E63E=0.000000,ResetOnDrop?_14_B5062806488C4B3CFA94728FF0322F7D=True)" "(BoundsType_3_295CD98E4D2862A6B4052790986A46EA=NewEnumerator0,LockSpecifiedValue_5_1E8FC7F64E9F7D85E5F24A85E78A6CFA=0.000000,Min_7_2A1EBA064A0EA8126606B59CD598994E=0.000000,Max_9_CD75696C42CE808B0A8BE1B2E7D1E63E=0.000000,ResetOnDrop?_14_B5062806488C4B3CFA94728FF0322F7D=True)" "(BoundsType_3_295CD98E4D2862A6B4052790986A46EA=NewEnumerator0,LockSpecifiedValue_5_1E8FC7F64E9F7D85E5F24A85E78A6CFA=0.000000,Min_7_2A1EBA064A0EA8126606B59CD598994E=0.000000,Max_9_CD75696C42CE808B0A8BE1B2E7D1E63E=0.000000,ResetOnDrop?_14_B5062806488C4B3CFA94728FF0322F7D=True)" "(BoundsType_3_295CD98E4D2862A6B4052790986A46EA=NewEnumerator0,LockSpecifiedValue_5_1E8FC7F64E9F7D85E5F24A85E78A6CFA=0.000000,Min_7_2A1EBA064A0EA8126606B59CD598994E=0.000000,Max_9_CD75696C42CE808B0A8BE1B2E7D1E63E=0.000000,HandAxisBinding_15_7791594F48674BE9C9DB8A83B34E0C75=NewEnumerator1,ResetOnDrop?_17_54497A634287FD69CB6B0ABA09C6D891=True)" "(BoundsType_3_295CD98E4D2862A6B4052790986A46EA=NewEnumerator0,LockSpecifiedValue_5_1E8FC7F64E9F7D85E5F24A85E78A6CFA=0.000000,Min_7_2A1EBA064A0EA8126606B59CD598994E=0.000000,Max_9_CD75696C42CE808B0A8BE1B2E7D1E63E=0.000000,HandAxisBinding_15_7791594F48674BE9C9DB8A83B34E0C75=NewEnumerator0,ResetOnDrop?_17_54497A634287FD69CB6B0ABA09C6D891=True)" "(BoundsType_3_295CD98E4D2862A6B4052790986A46EA=NewEnumerator0,LockSpecifiedValue_5_1E8FC7F64E9F7D85E5F24A85E78A6CFA=0.000000,Min_7_2A1EBA064A0EA8126606B59CD598994E=0.000000,Max_9_CD75696C42CE808B0A8BE1B2E7D1E63E=0.000000,HandAxisBinding_15_7791594F48674BE9C9DB8A83B34E0C75=NewEnumerator2,ResetOnDrop?_17_54497A634287FD69CB6B0ABA09C6D891=True)") true) (Utilities|Struct|MakeStruct_21_GripInfo "0.000000,0.000000,0.000000|0.000000,0.000000,0.000000|1.000000,1.000000,1.000000" false "NewEnumerator1" "NewEnumerator1" 1.0 "NewEnumerator3" "NewEnumerator4"))))))))

(fn ConstructionScript
  (|CallParentFunction)
  (bind _output_get (Variables|Default|Setidiot (- (.y (Transformation|GetSocketLocation (Variables|Default|GetSkeletalMesh) "palmsock")) (.y (Transformation|GetSocketLocation (Variables|Default|Get0_HandMesh) "palmsock")))))
  (Development|PrintString (Utilities|String|ToString(Float) _output_get)))

(fn NewFunction00
  (params (SCL :type STRUCT%2021%20Sub%20Component%20Logic%20Structure%20%28by%20ref%29))
  (bind _state (Utilities|Struct|BreakSTRUCT_21_SubComponentLogic SCL))
  (bind _subcomponentmap (Variables|Default|GetSubComponentMap))
  (bind _0_mesh_base (Variables|Default|Get0_Mesh_Base))
  (bind _hand (Utilities|Struct|BreakStruct_21_ComponentState _state))
  (bind _value (Utilities|Map|Find _subcomponentmap _0_mesh_base))
  (bind _hand_2 (Utilities|Struct|BreakStruct_21_ComponentState (.state _value)))
  (bind (_side _mc _ghost _solid) (Utilities|Struct|BreakStruct_21_HandSingularity _hand))
  (bind (_side_2 _mc_2 _ghost_2 _solid_2) (Utilities|Struct|BreakStruct_21_HandSingularity _hand_2))
  (bind _returnvalue (Math|Vector|GetForwardVector _ghost_2))
  (Utilities|IsValid _ghost_2
    (:Is%20Valid
      (Utilities|FlowControl|Sequence
        (:then_0
          (Utilities|FlowControl|Sequence
            (:then_0
              (Utilities|FlowControl|Sequence
                (:then_0
                  (Transformation|SetWorldRotation _solid_2 (Math|Rotator|MakeRotfromXY (Math|Vector|GetUnitDirection(Vector) (Transformation|GetSocketLocation _solid_2 "palmsock") (Transformation|GetSocketLocation _ghost "palmsock")) (Math|Vector|GetRightVector _ghost_2)) false false))
                (:then_1
                  ;[1 1 1] Keep Solid (frame) at ghost palm
                  (Transformation|AddWorldOffset _solid_2 (- (Transformation|GetSocketLocation _ghost_2 "palmsock") (Transformation|GetSocketLocation _solid_2 "palmsock")) false false))
                (:then_2
                  (Utilities|FlowControl|Sequence
                    (:then_2
                      (Transformation|SetWorldRotation _solid_2 (Math|Rotator|MakeRotfromXY (Math|Vector|GetUnitDirection(Vector) (Transformation|GetSocketLocation _solid_2 "palmsock") (Class|KismetMathLibrary|ProjectPointontoPlane (Transformation|GetSocketLocation _ghost "palmsock") (+ (Transformation|GetSocketLocation _ghost_2 "palmsock") (* _returnvalue 3e+01)) _returnvalue)) (Math|Vector|GetRightVector _ghost_2)) false false))))))))
        (:then_1
          ;[1 1 1] Fix Foregrip Solid Rotation
          (Transformation|SetWorldRotation _solid (Transformation|GetWorldRotation _ghost) false false))))))