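; BP_21_Item_Button is a pressable button item that configures itself through the parent class's sub-component system.
; On SCLogicSetup it adds one entry to SubComponentMap, keyed by its mesh and bundling the button root, mesh and highlighters.
; That entry enables Button manipulation with a single-axis travel limit and a default gravity mode.
; It has no other active logic, so interaction behavior is left outside this Blueprint.
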(event EventBeginPlay
  (|CallParentFunction) ; This node is disabled and will not be called.\nDrag off pins to build functionality.
)

(event Collision|EventActorBeginOverlap
  (params (OtherActor :type Actor%20Object%20Reference))
  (|CallParentFunction OtherActor) ; This node is disabled and will not be called.\nDrag off pins to build functionality.
)

(event EventTick
  (params (DeltaSeconds :type Float%20%28single-precision%29))
  (|CallParentFunction DeltaSeconds) ; This node is disabled and will not be called.\nDrag off pins to build functionality.
)

(event EventSCLogicSetup
  (bind _0_mesh_base1 (Variables|Default|Get0_Mesh_Base1))
  (Utilities|FlowControl|Sequence
    (:then_0
      (Utilities|FlowControl|Sequence
        (:then_0
          (Utilities|Map|Add (Variables|Default|GetSubComponentMap) _0_mesh_base1 (Utilities|Struct|MakeSTRUCT_21_SubComponentLogic (Utilities|Struct|MakeStruct_21_SubComponentObjects (Variables|Default|GetButtonRoot) _0_mesh_base1 0 (Variables|Default|Get0_Highlighter1) self 0 (Variables|Default|Getbadhilight)) (Utilities|Struct|MakeStruct_21_BasicComponentBehavior false "NewEnumerator2" false false false false false false false "NewEnumerator4") (Utilities|Struct|MakeStruct_21_ManipulationOptions false true false (Utilities|Struct|MakeStruct_ConstraintContainer "NewEnumerator1" (Utilities|Struct|MakeStruct_ButtonConstraints false false -1e+01 0.0 0.0 0.0 0.0 0.0 1e+01 0.0 "NewEnumerator2") "(BoundsType_3_295CD98E4D2862A6B4052790986A46EA=NewEnumerator0,LockSpecifiedValue_5_1E8FC7F64E9F7D85E5F24A85E78A6CFA=0.000000,Min_7_2A1EBA064A0EA8126606B59CD598994E=0.000000,Max_9_CD75696C42CE808B0A8BE1B2E7D1E63E=0.000000,ResetOnDrop?_14_B5062806488C4B3CFA94728FF0322F7D=True)" "(BoundsType_3_295CD98E4D2862A6B4052790986A46EA=NewEnumerator0,LockSpecifiedValue_5_1E8FC7F64E9F7D85E5F24A85E78A6CFA=0.000000,Min_7_2A1EBA064A0EA8126606B59CD598994E=0.000000,Max_9_CD75696C42CE808B0A8BE1B2E7D1E63E=0.000000,ResetOnDrop?_14_B5062806488C4B3CFA94728FF0322F7D=True)" "(BoundsType_3_295CD98E4D2862A6B4052790986A46EA=NewEnumerator0,LockSpecifiedValue_5_1E8FC7F64E9F7D85E5F24A85E78A6CFA=0.000000,Min_7_2A1EBA064A0EA8126606B59CD598994E=0.000000,Max_9_CD75696C42CE808B0A8BE1B2E7D1E63E=0.000000,ResetOnDrop?_14_B5062806488C4B3CFA94728FF0322F7D=True)" "(BoundsType_3_295CD98E4D2862A6B4052790986A46EA=NewEnumerator0,LockSpecifiedValue_5_1E8FC7F64E9F7D85E5F24A85E78A6CFA=0.000000,Min_7_2A1EBA064A0EA8126606B59CD598994E=0.000000,Max_9_CD75696C42CE808B0A8BE1B2E7D1E63E=0.000000,HandAxisBinding_15_7791594F48674BE9C9DB8A83B34E0C75=NewEnumerator1,ResetOnDrop?_17_54497A634287FD69CB6B0ABA09C6D891=True)" "(BoundsType_3_295CD98E4D2862A6B4052790986A46EA=NewEnumerator0,LockSpecifiedValue_5_1E8FC7F64E9F7D85E5F24A85E78A6CFA=0.000000,Min_7_2A1EBA064A0EA8126606B59CD598994E=0.000000,Max_9_CD75696C42CE808B0A8BE1B2E7D1E63E=0.000000,HandAxisBinding_15_7791594F48674BE9C9DB8A83B34E0C75=NewEnumerator0,ResetOnDrop?_17_54497A634287FD69CB6B0ABA09C6D891=True)" "(BoundsType_3_295CD98E4D2862A6B4052790986A46EA=NewEnumerator0,LockSpecifiedValue_5_1E8FC7F64E9F7D85E5F24A85E78A6CFA=0.000000,Min_7_2A1EBA064A0EA8126606B59CD598994E=0.000000,Max_9_CD75696C42CE808B0A8BE1B2E7D1E63E=0.000000,HandAxisBinding_15_7791594F48674BE9C9DB8A83B34E0C75=NewEnumerator2,ResetOnDrop?_17_54497A634287FD69CB6B0ABA09C6D891=True)")) "(PIckupOffset_12_5ACC95F941AD9A8A6DF52683A8A1737E=(Rotation=(X=0.000000,Y=0.000000,Z=0.000000,W=1.000000),Translation=(X=0.000000,Y=0.000000,Z=0.000000),Scale3D=(X=1.000000,Y=1.000000,Z=1.000000)),Reflection?_14_82FDBA9A41FCD8A869AF619B11559FC1=False,ReflectionAxis_5_B38E55D9470654EFAA6032A8FB977EA2=NewEnumerator1,GripPose_8_182C49484569F8C54CB1AC801069219F=NewEnumerator0,GripStrength_11_5991C4F74DE69A0BDED69A9884AC1F67=0.000000,CollisionOptions_17_BE4BF26943F7E980D264F4AFED50C411=NewEnumerator0,HandManipAttachment_21_1F4E67F34F599384CBFEA3842A4D5AE2=NewEnumerator0,Bone_24_5EC8B0144F76194A0232EAB1BD7F4EDE=\"palmsock\")" "(AttachType_3_18F51CA946EE74886BC1578FCBCCFACE=NewEnumerator0,AttachWholeActor?_28_6069CB334E12740D97A606BB9104A4EA=False,AttachOnDropOnly_20_BC81E01F47373AA4695193BE0479BE42=False,ShowHighlightOnMatch_22_66411197413AD07117DC5C882F635B4C=False,MyTag_5_C3CBA8364F2E2354D01FC3A6B7ABAAFA=\"\",SearchTag_7_80C2D3824149F98955FB71A1DE7E3145=\"\",Discriminate?_10_D63EBEB24AE3401D6437F7972806F8B8=False,FemaleAttachmentScene_14_7EF0E2F64379BDAC6ACE40857B7E6292=None,MaleAttachmentOffset_17_C7DC988A495FBCC69D62DAB7BE91F007=(Rotation=(X=0.000000,Y=0.000000,Z=0.000000,W=1.000000),Translation=(X=0.000000,Y=0.000000,Z=0.000000),Scale3D=(X=1.000000,Y=1.000000,Z=1.000000)),Highlighter_25_C4DEAC6340C67DC751E7A7A13D04AA3D=None,ProxWhenAttached?_30_45D2A9F4407F26BF46F4A293881E122C=False)" (Utilities|Struct|MakeStruct_21_ComponentState false false))))))))

(fn ConstructionScript
  (|CallParentFunction))