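; Pressable button actor in the MagicRoom that opens the Whitedoor when a VR or base pawn touches its Box trigger.
; A press lowers the Cube slightly, calls OpenWhite on the Whitedoor found in the level, then raises the Cube after a short delay.
; An Ispressed flag, set on any overlap before the pawn casts, blocks repeats until that sequence finishes.
; BeginPlay also runs the same press sequence.
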(event OnComponentBeginOverlap(Box)
  (params (OverlappedComponent :type Primitive%20Component%20Object%20Reference) (OtherActor :type Actor%20Object%20Reference) (OtherComp :type Primitive%20Component%20Object%20Reference) (OtherBodyIndex :type Integer) (bFromSweep :type Boolean) (SweepResult :type Hit%20Result%20Structure%20%28by%20ref%29))
  (bind _cube (Variables|Default|GetCube))
  (bind _cube_2 (Variables|Default|GetCube))
  (bind _returnvalue (Transformation|GetRelativeTransform _cube))
  (bind _returnvalue_2 (Transformation|GetRelativeTransform _cube_2))
  (if (not (Variables|Default|Getispressed))
    (Variables|Default|Setispressed true)
    (Utilities|FlowControl|Sequence
      (:then_0
        (Utilities|Casting|CastToBP_VRPawn OtherActor))
      (:then_1
        (Utilities|Casting|CastToBP_BasePawn OtherActor)))
    (Components|MoveComponentTo _cube_2 (- (.location _returnvalue_2) "0.000000,0.000000,5.000000") (.rotation _returnvalue_2) false false 0.2 false)
    (bind _returnvalue_3 (Actor|GetActorOfClass "/Game/MagicRoom/Blueprints/Whitedoor.Whitedoor_C"))
    (Default|OpenWhite _returnvalue_3)
    (Utilities|FlowControl|Delay 0.2)
    (Components|MoveComponentTo _cube (+ (.location _returnvalue) "0.000000,0.000000,5.000000") (.rotation _returnvalue) false false 0.2 false)
    (Variables|Default|Setispressed false)))

(event EventBeginPlay
  (bind _cube (Variables|Default|GetCube))
  (bind _cube_2 (Variables|Default|GetCube))
  (bind _returnvalue (Transformation|GetRelativeTransform _cube))
  (bind _returnvalue_2 (Transformation|GetRelativeTransform _cube_2))
  (Components|MoveComponentTo _cube_2 (- (.location _returnvalue_2) "0.000000,0.000000,5.000000") (.rotation _returnvalue_2) false false 0.2 false)
  (bind _returnvalue_3 (Actor|GetActorOfClass "/Game/MagicRoom/Blueprints/Whitedoor.Whitedoor_C"))
  (Default|OpenWhite _returnvalue_3)
  (Utilities|FlowControl|Delay 0.2)
  (Components|MoveComponentTo _cube (+ (.location _returnvalue) "0.000000,0.000000,5.000000") (.rotation _returnvalue) false false 0.2 false)
  (Variables|Default|Setispressed false))

(event Collision|EventActorBeginOverlap
  (params (OtherActor :type Actor%20Object%20Reference)))

(event EventTick
  (params (DeltaSeconds :type Float%20%28single-precision%29)))

(fn ConstructionScript)