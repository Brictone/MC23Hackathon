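; Right-hand cabinet door for the MagicRoom, swung open and shut by a VR motion controller.
; Grabbing within the handle sphere stores the hand and plays haptics, and releasing clears it and disables door physics.
; While unlocked and held, Tick sets the door's yaw from the hand-to-door look-at angle, clamped to a quarter turn.
; The lock events are empty, and the near-180-degree snap is unconnected.
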(event OnGrabbed(GrabComponent_R)
  (params (motion%20controller :type BP%20Motion%20Controller%20Object%20Reference))
  (bind _handlecollision_r (Variables|Default|GethandleCollision_R))
  ;[1 1 1] On Grabbed
  (if (Utilities|Operators|EqualEqual (Transformation|GetWorldLocation (Variables|/Game/CollaborativeViewer/Blueprints/Pawn/VR/BP_MotionController.BP_MotionController_C|GetHand motion%20controller)) (Transformation|GetWorldLocation _handlecollision_r) (Variables|/Script/Engine.SphereComponent|GetSphereRadius _handlecollision_r))
    (Variables|Default|SetHand (Variables|/Game/CollaborativeViewer/Blueprints/Pawn/VR/BP_MotionController.BP_MotionController_C|GetHand motion%20controller))
    (Class|PlayerController|PlayHapticEffect (Game|GetPlayerController 0) "/Game/MagicRoom/Haptic/GrabHapticEffect.GrabHapticEffect" (Default|GetHeldbyHand (Variables|Default|GetGrabComponent_R)) 1.0 false)))

(event OnDropped(GrabComponent_R)
  (params (Motion%20Controller :type BP%20Motion%20Controller%20Object%20Reference))
  ;[1 1 1] On Released
  (if (== (Variables|/Game/CollaborativeViewer/Blueprints/Pawn/VR/BP_MotionController.BP_MotionController_C|GetHand Motion%20Controller) (Variables|Default|GetHand))
    (Variables|Default|SetHand 0)
    (Physics|SetSimulatePhysics (Variables|Default|Getcabinet%20door%20R) false)))

(event Custom|isLocked_right_event
  (params (isLocked :type Boolean)))

(event Custom|isLocked_left_event
  (params (isLocked :type Boolean)))

(event EventBeginPlay)

(event Collision|EventActorBeginOverlap
  (params (OtherActor :type Actor%20Object%20Reference)))

(event EventTick
  (params (DeltaSeconds :type Float%20%28single-precision%29))
  (bind _hand (Variables|Default|GetHand))
  (bind _cabinet_door_r (Variables|Default|Getcabinet%20door%20R))
  ;[1 1 1] Cabinet Door Right tick
  (if (not (or (stale Custom|isLocked_right_event isLocked) (stale Custom|isLocked_left_event isLocked)))
    (Utilities|IsValid _hand
      (:Is%20Valid
        (Transformation|SetWorldRotation (Variables|Default|Getcabinet%20door%20R) (Math|Rotator|MakeRotator 0.0 0.0 (Math|Float|ClampAngle (- (.yaw (Math|Rotator|FindLookatRotation (Transformation|GetWorldLocation _hand) (Transformation|GetWorldLocation _cabinet_door_r))) 0.0) 9e+01 1.8e+02)) false false))
      (:Is%20Not%20Valid
        (if (Math|Float|NearlyEqual(Float) (.yaw (Transformation|GetWorldRotation _cabinet_door_r)) 1.8e+02 5.0)
          _)))))

(fn ConstructionScript)