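; VR main door for the magic room that locks and unlocks with an exit key and swings by a hand grab.
; A BP_ExitKey entering the handle collision toggles the lock and door physics, with a DoOnce that resets on end overlap and a haptic on unlock.
; While unlocked, Tick yaws the door toward the gripping hand within clamped limits.
; When released, a nearly closed door snaps shut.
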(event OnGrabbed(GrabComponent)
  (params (motion%20controller :type BP%20Motion%20Controller%20Object%20Reference))
  (bind _handlecollision (Variables|Default|GethandleCollision))
  ;[1 1 1] On Grabbed
  (if (Utilities|Operators|EqualEqual (Transformation|GetWorldLocation (Variables|/Game/CollaborativeViewer/Blueprints/Pawn/VR/BP_MotionController.BP_MotionController_C|GetHand motion%20controller)) (Transformation|GetWorldLocation _handlecollision) (Variables|/Script/Engine.SphereComponent|GetSphereRadius _handlecollision))
    (Variables|Default|SetHand (Variables|/Game/CollaborativeViewer/Blueprints/Pawn/VR/BP_MotionController.BP_MotionController_C|GetHand motion%20controller))
    (Class|PlayerController|PlayHapticEffect (Game|GetPlayerController 0) "/Game/MagicRoom/Haptic/GrabHapticEffect.GrabHapticEffect" (Default|GetHeldbyHand (Variables|Default|GetGrabComponent)) 1.0 false)))

(event OnDropped(GrabComponent)
  (params (Motion%20Controller :type BP%20Motion%20Controller%20Object%20Reference))
  ;[1 1 1] On Released
  (if (== (Variables|/Game/CollaborativeViewer/Blueprints/Pawn/VR/BP_MotionController.BP_MotionController_C|GetHand Motion%20Controller) (Variables|Default|GetHand))
    (Variables|Default|SetHand 0)))

(event OnComponentBeginOverlap(handleCollision)
  (params (OverlappedComponent :type Primitive%20Component%20Object%20Reference) (OtherActor :type Actor%20Object%20Reference) (OtherComp :type Primitive%20Component%20Object%20Reference) (OtherBodyIndex :type Integer) (bFromSweep :type Boolean) (SweepResult :type Hit%20Result%20Structure%20%28by%20ref%29))
  (bind _door (Variables|Default|Getdoor))
  ;[1 1 1] check if key
  (bind _handlecollision (Variables|Default|GethandleCollision)
    (:then
      (for _array_element (Collision|GetOverlappingActors _handlecollision "/Game/MagicRoom/Blueprints/BP_ExitKey.BP_ExitKey_C" :!class /Script/Engine.PrimitiveComponent)
        (if (Utilities|Enum|Equal(Enum) (Utilities|GetDisplayName _array_element) "BP_ExitKey")
          (Utilities|FlowControl|DoOnce false
            (:Completed
              (bind _asbp_exit_key (Utilities|Casting|CastToBP_ExitKey _array_element))
              (Variables|Default|Setkey _asbp_exit_key)
              (if (Variables|Default|GetisLocked)
                (Variables|Default|SetisLocked false)
                (Physics|SetSimulatePhysics _door true)
                ;[1 1 1] Play haptic in hand holding key
                (Class|PlayerController|PlayHapticEffect (Game|GetPlayerController 0) "/Game/MagicRoom/Haptic/GrabHapticEffect.GrabHapticEffect" (Default|GetHeldbyHand (Variables|/Game/MagicRoom/Blueprints/BP_ExitKey.BP_ExitKey_C|GetGrabComponent (Variables|Default|Getkey))) 1.0 false)
                (else
                  (Variables|Default|SetisLocked true)
                  (Physics|SetSimulatePhysics _door false))))))))
    (:else)))

(event OnComponentEndOverlap(handleCollision)
  (params (OverlappedComponent :type Primitive%20Component%20Object%20Reference) (OtherActor :type Actor%20Object%20Reference) (OtherComp :type Primitive%20Component%20Object%20Reference) (OtherBodyIndex :type Integer))
  (bind _door (Variables|Default|Getdoor))
  ;[1 1 1] check if key
  (Utilities|FlowControl|DoOnce false) ; enters at Reset
)

(event EventBeginPlay)

(event Collision|EventActorBeginOverlap
  (params (OtherActor :type Actor%20Object%20Reference)))

(event EventTick
  (params (DeltaSeconds :type Float%20%28single-precision%29))
  (bind _hand (Variables|Default|GetHand))
  (bind _door (Variables|Default|Getdoor))
  ;[1 1 1] Comment
  (if (not (Variables|Default|GetisLocked))
    (Utilities|IsValid _hand
      (:Is%20Valid
        (Transformation|SetWorldRotation (Variables|Default|Getdoor) (Math|Rotator|MakeRotator 0.0 0.0 (Math|Float|ClampAngle (- (.yaw (Math|Rotator|FindLookatRotation (Transformation|GetWorldLocation _hand) (Transformation|GetWorldLocation _door))) 9e+01) -9e+01 9e+01)) false false))
      (:Is%20Not%20Valid
        (if (Math|Float|NearlyEqual(Float) (.yaw (Transformation|GetWorldRotation _door)) 0.0 5.0)
          (Transformation|SetWorldRotation _door "0, 0, 0" false false))))))

(fn ConstructionScript)