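; Left cabinet door for VR in the Magic Room, swung open and shut by a motion-controller hand.
; Grabbing within the handle's collision sphere stores the hand and plays haptics; releasing clears it and turns off door physics.
; While both left and right latches are unlocked, Tick yaws the door toward the held hand within a clamped arc.
; The near-closed check does nothing, its snap rotation is unwired, and Tick prints latch debug text.
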(event OnDropped(GrabComponent_L)
  (params (Motion%20Controller :type BP%20Motion%20Controller%20Object%20Reference))
  ;[1 1 1] On Released
  (if (== (Variables|/Game/CollaborativeViewer/Blueprints/Pawn/VR/BP_MotionController.BP_MotionController_C|GetHand Motion%20Controller) (Variables|Default|GetHand))
    (Variables|Default|SetHand 0)
    (Physics|SetSimulatePhysics (Variables|Default|Getcabinet%20door%20L) false)))

(event OnGrabbed(GrabComponent_L)
  (params (motion%20controller :type BP%20Motion%20Controller%20Object%20Reference))
  (bind _handlecollision_l (Variables|Default|GethandleCollision_L))
  ;[1 1 1] On Grabbed
  (if (Utilities|Operators|EqualEqual (Transformation|GetWorldLocation (Variables|/Game/CollaborativeViewer/Blueprints/Pawn/VR/BP_MotionController.BP_MotionController_C|GetHand motion%20controller)) (Transformation|GetWorldLocation _handlecollision_l) (Variables|/Script/Engine.SphereComponent|GetSphereRadius _handlecollision_l))
    (Variables|Default|SetHand (Variables|/Game/CollaborativeViewer/Blueprints/Pawn/VR/BP_MotionController.BP_MotionController_C|GetHand motion%20controller))
    (Class|PlayerController|PlayHapticEffect (Game|GetPlayerController 0) "/Game/MagicRoom/Haptic/GrabHapticEffect.GrabHapticEffect" (Default|GetHeldbyHand (Variables|Default|GetGrabComponent_L)) 1.0 false)))

(event EventBeginPlay)

(event Collision|EventActorBeginOverlap
  (params (OtherActor :type Actor%20Object%20Reference)))

(event EventTick
  (params (DeltaSeconds :type Float%20%28single-precision%29))
  (bind _hand (Variables|Default|GetHand))
  (bind _cabinetlatch_left (Variables|Default|GetcabinetLatch_Left))
  (bind _cabinet_door_l (Variables|Default|Getcabinet%20door%20L))
  (bind _islocked_left (Variables|/Game/MagicRoom/Blueprints/cabinetLatch_Left.cabinetLatch_Left_C|GetisLocked_Left _cabinetlatch_left))
  ;[1 1 1] Cabinet Door Left tick
  (Development|PrintString (Utilities|String|Append "left latch?" (Utilities|String|ToString(Boolean) _islocked_left)))
  (if (not (or _islocked_left (Variables|/Game/MagicRoom/Blueprints/cabinetLatch_Right.cabinetLatch_Right_C|GetisLocked_Right (Variables|Default|GetcabinetLatch_Right))))
    (Utilities|IsValid _hand
      (:Is%20Valid
        (Transformation|SetWorldRotation (Variables|Default|Getcabinet%20door%20L) (Math|Rotator|MakeRotator 0.0 0.0 (Math|Float|ClampAngle (- (.yaw (Math|Rotator|FindLookatRotation (Transformation|GetWorldLocation _hand) (Transformation|GetWorldLocation _cabinet_door_l))) -1.8e+02) -1.8e+02 -9e+01)) false false))
      (:Is%20Not%20Valid
        (if (Math|Float|NearlyEqual(Float) (.yaw (Transformation|GetWorldRotation _cabinet_door_l)) 1.8e+02 5.0)
          _)))))

(fn ConstructionScript)