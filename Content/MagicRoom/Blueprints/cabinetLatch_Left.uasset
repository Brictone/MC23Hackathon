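; VR sliding left latch for a cabinet, controlling the left-side lock state on both cabinet doors.
; Grabbing within the handle's collision radius stores the hand and plays haptics, while dropping clears it and disables latch physics.
; Tick slides the held latch along a clamped, hard-coded world X range.
; When not held, a latch near the upper limit snaps there and unlocks both doors, otherwise it locks them.
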(event OnDropped(GrabComponent_L)
  (params (Motion%20Controller :type BP%20Motion%20Controller%20Object%20Reference))
  ;[1 1 1] On Released
  (if (== (Variables|/Game/CollaborativeViewer/Blueprints/Pawn/VR/BP_MotionController.BP_MotionController_C|GetHand Motion%20Controller) (Variables|Default|GetHand))
    (Variables|Default|SetHand 0)
    (Physics|SetSimulatePhysics (Variables|Default|GetCabinetLatch_L) false)))

(event OnGrabbed(GrabComponent_L)
  (params (motion%20controller :type BP%20Motion%20Controller%20Object%20Reference))
  (bind _handlecollision_l (Variables|Default|GethandleCollision_L))
  ;[1 1 1] On Grabbed
  (if (Utilities|Operators|EqualEqual (Transformation|GetWorldLocation (Variables|/Game/CollaborativeViewer/Blueprints/Pawn/VR/BP_MotionController.BP_MotionController_C|GetHand motion%20controller)) (Transformation|GetWorldLocation _handlecollision_l) (Variables|/Script/Engine.SphereComponent|GetSphereRadius _handlecollision_l))
    (Variables|Default|SetHand (Variables|/Game/CollaborativeViewer/Blueprints/Pawn/VR/BP_MotionController.BP_MotionController_C|GetHand motion%20controller))
    (Class|PlayerController|PlayHapticEffect (Game|GetPlayerController 0) "/Game/MagicRoom/Haptic/GrabHapticEffect.GrabHapticEffect" (Default|GetHeldbyHand (Variables|Default|GetGrabComponent_L)) 1.0 false)))

(event EventBeginPlay)

(event Collision|EventActorBeginOverlap
  (params (OtherActor :type Actor%20Object%20Reference)))

(event EventTick
  (params (DeltaSeconds :type Float%20%28single-precision%29))
  (bind _hand (Variables|Default|GetHand))
  (bind _cabinetlatch_l (Variables|Default|GetCabinetLatch_L))
  (bind _cabinetdoorl_right (Variables|Default|GetcabinetDoorl_Right))
  (bind _cabinetdoor_left (Variables|Default|GetcabinetDoor_Left))
  (bind _returnvalue (Transformation|GetWorldLocation _cabinetlatch_l))
  ;[1 1 1] Cabinet Door Left tick
  (Utilities|IsValid _hand
    (:Is%20Valid
      (Transformation|SetWorldLocation (Variables|Default|GetCabinetLatch_L) (Math|Vector|MakeVector (Math|Float|Clamp(Float) (.x (Transformation|GetWorldLocation _hand)) 5e+01 55.0) (.y _returnvalue) (.z _returnvalue)) false false))
    (:Is%20Not%20Valid
      (if (Math|Float|NearlyEqual(Float) (.x _returnvalue) 55.0 1.0)
        (Transformation|SetWorldLocation _cabinetlatch_l (Math|Vector|MakeVector 55.0 (.y _returnvalue) (.z _returnvalue)) false false)
        (if true
          (Utilities|FlowControl|Sequence
            (:then_0
              (Default|IsLockedLeftEvent _cabinetdoorl_right false))
            (:then_1
              (Default|IsLockedLeftEvent _cabinetdoor_left false))))
        (else
          (Utilities|FlowControl|Sequence
            (:then_0
              (Default|IsLockedLeftEvent _cabinetdoorl_right true))
            (:then_1
              (Default|IsLockedLeftEvent _cabinetdoor_left true))))))))

(fn ConstructionScript)