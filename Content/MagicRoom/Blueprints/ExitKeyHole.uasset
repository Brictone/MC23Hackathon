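; ExitKeyHole is a keyhole Blueprint meant to detect an exit key, though its detection is unfinished.
; BeginPlay caches world-space start and end points from two spline points.
; While no valid Key is set, Tick runs a sphere overlap at the start point, but the loop body is empty.
; The logic to cast to BP_ExitKey, store it and detach it is disconnected and never runs.
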(event EventBeginPlay
  (bind _spline (Variables|Default|GetSpline))
  (Variables|Default|SetstartPoint (Spline|GetLocationatSplinePoint _spline 1 "World"))
  (Variables|Default|SetendPoint (Spline|GetLocationatSplinePoint _spline 0 "World")))

(event EventTick
  (params (DeltaSeconds :type Float%20%28single-precision%29))
  (Utilities|IsValid (Variables|Default|Getkey)
    (:Is%20Not%20Valid
      ;[1 1 1] detect key
      (bind _outactors (Collision|SphereOverlapActors (Variables|Default|GetstartPoint) 2e+01 (Utilities|Array|MakeArray "ObjectTypeQuery2") 0))
      (bind _array_element (Utilities|Array|ForEachLoopwithBreak _outactors)))))

(fn ConstructionScript)