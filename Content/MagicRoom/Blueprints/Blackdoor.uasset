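; Blackdoor is a door actor in MagicRoom that appears and disappears by changing the visibility of its Cube component.
; Shortly after BeginPlay, it shows the Cube if the player's BP_BasePawn has Isblack set.
; The OpenBlack event uses a FlipFlop to alternate between hiding and showing the Cube, starting with hide, regardless of its current state.
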(event Custom|OpenBlack
  (Utilities|FlowControl|FlipFlop
    (:A
      (Rendering|SetVisibility (Variables|Default|GetCube) false false))
    (:B
      (Rendering|SetVisibility (Variables|Default|GetCube) true false))))

(event EventBeginPlay
  (Utilities|FlowControl|Delay 0.1)
  (bind _asbp_base_pawn (Utilities|Casting|CastToBP_BasePawn (Game|Player|GetPlayerPawn 0)))
  (if (Variables|/Game/CollaborativeViewer/Blueprints/Pawn/BP_BasePawn.BP_BasePawn_C|GetIsblack _asbp_base_pawn)
    (Rendering|SetVisibility (Variables|Default|GetCube) true false)))

(event Collision|EventActorBeginOverlap
  (params (OtherActor :type Actor%20Object%20Reference)))

(event EventTick
  (params (DeltaSeconds :type Float%20%28single-precision%29)))

(fn ConstructionScript)