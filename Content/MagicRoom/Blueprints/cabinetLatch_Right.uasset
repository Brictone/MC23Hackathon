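; Right-hand latch for a VR cabinet in the magic room that locks and unlocks both cabinet doors.
; Grabbing near the handle's collision sphere stores the controller's hand and plays haptics; dropping clears it.
; While held, Tick makes the latch follow the hand along a clamped, hard-coded world X range.
; When not held, Tick snaps a latch near the minimum to it and unlocks both doors, otherwise locks both.
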(event OnGrabbed(GrabComponent_R)
  (params (motion%20controller :type BP%20Motion%20Controller%20Object%20Reference))
  (bind _handlecollision_r (Variables|Default|GethandleCollision_R))
  ;[1 1 1] On Grabbed
  (if (Utilities|Operators|EqualEqual (Transformation|GetWorldLocation (Variables|/Game/CollaborativeViewer/Blueprints/Pawn/VR/BP_MotionController.BP_MotionController_C|GetHand motion%20controller)) (Transformation|GetWorldLocation _handlecollision_r) (Variables|/Script/Engine.SphereComponent|GetSphereRadius _handlecollision_r))
    (Variables|Default|SetHand (Variables|/Game/CollaborativeViewer/Blueprints/Pawn/VR/BP_MotionController.BP_MotionController_C|GetHand motion%20controller))
    (Class|PlayerController|PlayHapticEffect (Game|GetPlayerController 0) "/Game/MagicRoom/Haptic/GrabHapticEffect.GrabHapticEffect" (Default|GetHeldbyHand (Variables|Default|GetGrabComponent_R)) 1.0 false)))

(event OnDropped(GrabComponent_R)
  (params (Motion%20Controller :type BP%20Motion%20Controller%20Object%20Reference))
  ;[1 1 1] On Released
  (if (== (Variables|/Game/CollaborativeViewer/Blueprints/Pawn/VR/BP_MotionController.BP_MotionController_C|GetHand Motion%20Controller) (Variables|Default|GetHand))
    (Variables|Default|SetHand 0)
    (Physics|SetSimulatePhysics (Variables|Default|GetCabinetLatch_R) false)))

(event EventBeginPlay)

(event Collision|EventActorBeginOverlap
  (params (OtherActor :type Actor%20Object%20Reference)))

(event EventTick
  (params (DeltaSeconds :type Float%20%28single-precision%29))
  (bind _cabinetdoor_righ (Variables|Default|GetcabinetDoor_Righ))
  (bind _cabinetlatch_r (Variables|Default|GetCabinetLatch_R))
  (bind _hand (Variables|Default|GetHand))
  (bind _cabinetdoor_left (Variables|Default|GetcabinetDoor_Left))
  (bind _returnvalue (Transformation|GetWorldLocation _cabinetlatch_r))
  ;[1 1 1] Cabinet Door Left tick
  (Utilities|IsValid _hand
    (:Is%20Valid
      (Transformation|SetWorldLocation (Variables|Default|GetCabinetLatch_R) (Math|Vector|MakeVector (Math|Float|Clamp(Float) (.x (Transformation|GetWorldLocation _hand)) 2e+01 25.0) (.y _returnvalue) (.z _returnvalue)) false false))
    (:Is%20Not%20Valid
      (if (Math|Float|NearlyEqual(Float) (.x _returnvalue) 2e+01 1.0)
        (Transformation|SetWorldLocation _cabinetlatch_r (Math|Vector|MakeVector 2e+01 (.y _returnvalue) (.z _returnvalue)) false false)
        (if true
          (Utilities|FlowControl|Sequence
            (:then_0
              (Default|IsLockedRightEvent _cabinetdoor_righ false))
            (:then_1
              (Default|IsLockedRightEvent _cabinetdoor_left false))))
        (else
          (Utilities|FlowControl|Sequence
            (:then_0
              (Default|IsLockedRightEvent _cabinetdoor_righ true))
            (:then_1
              (Default|IsLockedRightEvent _cabinetdoor_left true))))))))

(fn ConstructionScript)